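; KGCharacterBase is a base character with sword melee, magic projectile attacks, health, flinching and death.
; It spawns a socketed sword on BeginPlay and sets a hair colour material parameter on construction.
; Melee chains attacks through montage sections, while magic plays a shoot montage, with projectile spawning in a separate event.
; Damage triggers small or big flinches depending on attack montage state, skipped during AttackMoves sections, or death and destruction.
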(event Custom|UsePrimaryAttack
  (CallFunction|TryMelee))

(event Custom|TryMelee
  (bind _mesh (Variables|Character|GetMesh))
  (bind _returnvalue (Components|SkeletalMesh|GetAnimInstance _mesh))
  (bind _returnvalue_2 (Animation|Montage|MontageGetCurrentSection _returnvalue "/Game/Assets/Knight/KnightAttackMontage.KnightAttackMontage"))
  (if (not (Variables|Default|GetIsFlinching))
    (if (Class|AnimInstance|MontageIsActive _returnvalue "/Game/Assets/Knight/KnightAttackMontage.KnightAttackMontage")
      (switch name _returnvalue_2
        (:Attack1
          (Class|AnimInstance|MontageSetNextSection _returnvalue _returnvalue_2 "Attack2" "/Game/Assets/Knight/KnightAttackMontage.KnightAttackMontage")))
      (else
        (Animation|PlayAnimMontage "/Game/Assets/Knight/KnightAttackMontage.KnightAttackMontage" 1.0 "Attack1")))))

(event Custom|TryMagic
  (if (not (Variables|Default|GetIsFlinching))
    (Animation|PlayAnimMontage "/Game/Assets/Knight/PlayerShoot.PlayerShoot" 1.0 "None")))

(event Custom|CreateSword
  (bind _returnvalue (Game|SpawnActorfromClass "/Game/BluePrints/BaseSword.BaseSword_C" (Transformation|GetActorTransform) "Undefined" 0 0))
  (bind _output_get (Variables|Default|SetWeapon _returnvalue))
  (Transformation|AttachComponentToComponent _output_get (Variables|Character|GetMesh) "Sword_Socket" "SnapToTarget" "SnapToTarget" "SnapToTarget" false))

(event Custom|LaunchMagicProjectile
  (Game|SpawnActorfromClass "/Game/BluePrints/KGProjectileBase.KGProjectileBase_C" (Transformation|GetWorldTransform (Variables|Default|GetProjectileFirePosition)) "Undefined" 0 self))

(event EventBeginPlay
  (bind (_weapon _health _attackmoves _isflinching _isdead) (Utilities|GetClassDefaults "KGCharacterBase_C"))
  (CallFunction|CreateSword)
  (Variables|Default|SetHealth _health)
  (Variables|Default|SetIsFlinching _isflinching)
  (Variables|Default|SetIsDead _isdead))

(event Collision|EventActorBeginOverlap
  (params (OtherActor :type Actor%20Object%20Reference)))

(event EventTick
  (params (DeltaSeconds :type Float%20%28single-precision%29)))

(event Game|Damage|EventAnyDamage
  (params (Damage :type Float%20%28single-precision%29) (DamageType :type Damage%20Type%20Object%20Reference) (InstigatedBy :type Controller%20Object%20Reference) (DamageCauser :type Actor%20Object%20Reference))
  (bind _mesh (Variables|Character|GetMesh))
  (bind _returnvalue (Components|SkeletalMesh|GetAnimInstance _mesh))
  (bind _output_get (Variables|Default|SetHealth (- (Variables|Default|GetHealth) Damage)))
  (if (<= _output_get 0.0)
    (Utilities|FlowControl|DoOnce false
      (:Completed
        (Variables|Default|SetIsFlinching true)
        (Variables|Default|SetIsDead true)
        (Pawn|Components|CharacterMovement|DisableMovement (Variables|Character|GetCharacterMovement))
        (bind _returnvalue_2 (Animation|PlayAnimMontage "/Game/Assets/Knight/PlayerDeathMontage.PlayerDeathMontage" 1.0 "None"))
        (Utilities|FlowControl|Delay _returnvalue_2)
        (Actor|DestroyActor (Variables|Default|GetWeapon))
        (Actor|DestroyActor)))
    (else
      (Variables|Default|SetIsFlinching true)
      (if (Class|AnimInstance|MontageIsActive _returnvalue "/Game/Assets/Knight/KnightAttackMontage.KnightAttackMontage") ; Is attack montage playing
        (if (Utilities|Array|ContainsItem (Variables|Default|GetAttackMoves) (Animation|Montage|MontageGetCurrentSection _returnvalue "/Game/Assets/Knight/KnightAttackMontage.KnightAttackMontage")) ; big finch happens whilst in recovery
          (Variables|Default|SetIsFlinching false)
          (else
            (bind _returnvalue_3 (Animation|PlayAnimMontage "/Game/Assets/Knight/PlayerFlinch.PlayerFlinch" 1.0 "FlinchBig"))
            (Utilities|FlowControl|Delay _returnvalue_3)
            (Variables|Default|SetIsFlinching false)))
        (else
          (bind _returnvalue_4 (Animation|PlayAnimMontage "/Game/Assets/Knight/PlayerFlinch.PlayerFlinch" 1.0 "FlinchSmall"))
          (Utilities|FlowControl|Delay _returnvalue_4)
          (Variables|Default|SetIsFlinching false))))))

(fn ConstructionScript
  (bind _returnvalue (Rendering|Material|CreateDynamicMaterialInstance (Variables|Character|GetMesh) 0 0 "None" :!class /Script/Engine.PrimitiveComponent))
  (Rendering|Material|SetVectorParameterValue _returnvalue "HairColour" (Variables|Default|GetHairColour) :!class /Script/Engine.MaterialInstanceDynamic))