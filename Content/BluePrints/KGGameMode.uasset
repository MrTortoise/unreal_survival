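; KGGameMode is a game mode that runs wave-based AI enemy spawning.
; At start it loads the current wave's class list into a shuffled queue, and a looping timer spawns the next entry at a random PlayerStart.
; Each enemy's destruction triggers a check that advances to the next wave once the queue is empty and only one KGAIControllerBase remains.
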(event Custom|SpawnEnemy
  (if (> (Utilities|Array|Length (Variables|Default|GetCurrentQueue)) 0) ; spawn more for current wave?
    (bind _outactors (Actor|GetAllActorsOfClass "/Script/Engine.PlayerStart")) ; pick a spawn point
    (bind _returnvalue (AI|SpawnAIFromClass (Utilities|Array|Get(acopy) (Variables|Default|GetCurrentQueue)) 0 (Transformation|GetActorLocation (Utilities|Array|Get(acopy) _outactors (Math|Random|RandomInteger (Utilities|Array|Length _outactors)))) (Transformation|GetActorRotation (Utilities|Array|Get(acopy) _outactors (Math|Random|RandomInteger (Utilities|Array|Length _outactors)))) false 0))
    (Utilities|Array|RemoveIndex (Variables|Default|GetCurrentQueue))
    (Game|BindEventtoOnDestroyed _returnvalue (delegate Custom|CheckWaveComplete))))

(event Custom|StartNewWave
  (Math|Integer|IncrementInt (Variables|Default|GetwaveIndex)
    (:%20%20
      (bind _output_get (Variables|Default|SetCurrentQueue (.classtospawn (Utilities|Array|Get(acopy) (Variables|Default|GetWaves) (Variables|Default|GetwaveIndex)))))
      (Utilities|Array|Shuffle _output_get))))

(event Custom|CheckWaveComplete
  (params (DestroyedActor :type Actor%20Object%20Reference))
  (if (== (Utilities|Array|Length (Variables|Default|GetCurrentQueue)) 0) ; Has Queue Finished Spawning?
    (bind _outactors (Actor|GetAllActorsOfClass "/Game/BluePrints/KGAIControllerBase.KGAIControllerBase_C"))
    (if (== (Utilities|Array|Length _outactors) 1) ; Are all AI dead
      (CallFunction|StartNewWave))))

(event Custom|ResetGame
  (bind _output_get (Variables|Default|SetCurrentQueue (.classtospawn (Utilities|Array|Get(acopy) (Variables|Default|GetWaves) (Variables|Default|GetwaveIndex)))))
  (Utilities|Array|Shuffle _output_get))

(event EventBeginPlay
  (Utilities|Time|SetTimerbyEvent (delegate Custom|SpawnEnemy) 1.0 true)
  (CallFunction|ResetGame))

(event EventTick
  (params (DeltaSeconds :type Float%20%28single-precision%29)))

(fn ConstructionScript)